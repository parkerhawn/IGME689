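; Pillar actor that rewards a player who reaches it while carrying, by adding time to the Timer.
; Each Tick it polls for overlapping BP_FirstPersonCharacter actors and checks IsCarrying on the first one found.
; When that is true it destroys itself and adds 30 to Time on the first top-level Timer widget, leaving IsCarrying unchanged.
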(event `self.ReceiveTick`
  (params (DeltaSeconds :type "Float (single-precision)"))
  (bind _overlappingactors (`self.GetOverlappingActors` "/Game/FirstPerson/Blueprints/BP_FirstPersonCharacter.BP_FirstPersonCharacter_C"))
  (for _ _overlappingactors
    (if (`/Game/FirstPerson/Blueprints/BP_FirstPersonCharacter.isCarrying` (`|GetArrayItem` _overlappingactors))
      (`self.K2_DestroyActor`)
      (bind _foundwidgets (`WidgetBlueprintLibrary.GetAllWidgetsOfClass` "/Game/Blueprints/Timer.Timer_C"))
      (bind _output (`|GetArrayItem` _foundwidgets))
      (set `/Game/Blueprints/Timer.Time` (+ (`/Game/Blueprints/Timer.Time` _output) 30.0) _output))))

(fn `UserConstructionScript`)