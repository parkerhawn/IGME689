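; Mini-map Blueprint that writes an ArcGIS position to the first-person character's ArcGISLocation every tick.
; On BeginPlay it casts player controller 0, rather than its pawn, to BP_FirstPersonCharacter and caches that character's ArcGISLocationComponent.
; Tick reads X and Y from the cached component, builds a WGS84 point without passing Z, and sets it on ArcGISLocation.
; No map rendering or UI logic is present.
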(event `self.ReceiveBeginPlay`
  (bind _asbp_first_person_character (cast `/Game/FirstPerson/Blueprints/BP_FirstPersonCharacter` (`GameplayStatics.GetPlayerController` 0)))
  (bind _output_get (set `self.BP First Person Character` _asbp_first_person_character))
  (set `self.CharacterLocationComponent` (`self.GetComponentByClass` _output_get "/Script/ArcGISMapsSDK.ArcGISLocationComponent")))

(event `self.ReceiveTick`
  (params (DeltaSeconds :type "Float (single-precision)"))
  (bind _returnvalue (`ArcGISLocationComponent.GetPosition` (`self.CharacterLocationComponent`)))
  (bind _returnvalue_2 (`ArcGISPoint.GetX` _returnvalue))
  (bind _returnvalue_3 (`ArcGISPoint.GetY` _returnvalue))
  (bind _returnvalue_4 (`ArcGISSpatialReference.WGS84`))
  (bind _returnvalue_5 (`ArcGISPoint.CreateArcGISPointWithXYZSpatialReference` _returnvalue_2 _returnvalue_3 0.0 _returnvalue_4))
  (`ArcGISLocationComponent.SetPosition` (`/Game/FirstPerson/Blueprints/BP_FirstPersonCharacter.ArcGISLocation` (`self.BP First Person Character`)) _returnvalue_5))

(fn `UserConstructionScript`)