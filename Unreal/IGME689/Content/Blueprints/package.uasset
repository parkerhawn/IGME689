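; A package actor that shows a floating pickup prompt when the first-person player can pick it up.
; Every tick it looks up BP_FirstPersonCharacter and shows PickupText only while the player overlaps DisplayRadius and is not already carrying.
; The visible text billboards toward the player by copying the camera rotation with yaw turned half a circle.
; The graph handles only the prompt, with no pickup logic.
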(event `self.ReceiveTick`
  (params (DeltaSeconds :type "Float (single-precision)"))
  (bind _player (`self.Player`))
  (bind _pickuptext (`self.PickupText`))
  (bind _returnvalue (`GameplayStatics.GetActorOfClass` "/Game/FirstPerson/Blueprints/BP_FirstPersonCharacter.BP_FirstPersonCharacter_C"))
  (bind _output_get (set `self.Player` _returnvalue))
  (if (or (`/Game/FirstPerson/Blueprints/BP_FirstPersonCharacter.isCarrying` _player) (not (`PrimitiveComponent.IsOverlappingActor` (`self.displayRadius`) _player)))
    (`SceneComponent.SetVisibility` _pickuptext false false)
    (else
      (`SceneComponent.SetVisibility` _pickuptext true false)
      (bind (_returnvalue_roll _returnvalue_pitch _returnvalue_yaw) (`KismetMathLibrary.BreakRotator` (`SceneComponent.K2_GetComponentRotation` (`/Game/FirstPerson/Blueprints/BP_FirstPersonCharacter.FirstPersonCamera` _output_get))))
      (`SceneComponent.K2_SetWorldRotation` _pickuptext (`KismetMathLibrary.MakeRotator` _returnvalue_roll _returnvalue_pitch (+ _returnvalue_yaw -180.0)) false false))))

(fn `UserConstructionScript`)